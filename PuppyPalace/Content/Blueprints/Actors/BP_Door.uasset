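; BP_Door is a door actor that reacts when a Pawn enters its Trigger component.
; The first overlap sets IsOpen and plays the TL_Open timeline; the graph shows no timeline update logic and no closing path.
; OverlapCount increments on entry but resets to zero when any Pawn leaves, followed by an empty check.
; An unconnected clamp on OverlapCount never runs.
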(event `self.Trigger.OnComponentEndOverlap`
  (params (OverlappedComponent :type "PrimitiveComponent Object Reference") (OtherActor :type "Actor Object Reference") (OtherComp :type "PrimitiveComponent Object Reference") (OtherBodyIndex :type Integer))
  (cast `Pawn` OtherActor)
  (set `self.OverlapCount` 0)
  (if (== (`self.OverlapCount`) 0)
    _))

(event `self.Trigger.OnComponentBeginOverlap`
  (params (OverlappedComponent :type "PrimitiveComponent Object Reference") (OtherActor :type "Actor Object Reference") (OtherComp :type "PrimitiveComponent Object Reference") (OtherBodyIndex :type Integer) (bFromSweep :type Boolean) (SweepResult :type "HitResult Structure (by ref)"))
  (cast `Pawn` OtherActor)
  (set `self.OverlapCount` (+ (`self.OverlapCount`) 1))
  (if (not (`self.bIsOpen`))
    (set `self.bIsOpen` true)
    (`Timeline|TL_Open`)))

(fn `UserConstructionScript`)